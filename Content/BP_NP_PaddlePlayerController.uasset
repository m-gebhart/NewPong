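; Player controller Blueprint for a two-paddle game that drives each paddle's layered music from the score.
; On game start, it initializes the BpC_MusicTrack component on both paddles with each player's selected soundtrack.
; When a player scores, the parity of the score difference decides the layer change: odd queues an added layer for the scorer, even queues a removed layer for the opponent.
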(event EventStartGameBP
  (Default|InitializeTrack (Actor|GetComponentbyClass (Variables|Default|GetPaddle) "/Game/BpC_MusicTrack.BpC_MusicTrack_C") (Utilities|Select :Index (Variables|Default|GetP1Soundtrack) :Option%200 "Track_01" :Option%201 "Track_01" :Option%202 "Track_02" :Option%203 "Track_03"))
  (Default|InitializeTrack (Actor|GetComponentbyClass (Variables|Default|GetLeftPaddle) "/Game/BpC_MusicTrack.BpC_MusicTrack_C") (Utilities|Select :Index (Variables|Default|GetP2Soundtrack) :Option%200 "Track_01" :Option%201 "Track_01" :Option%202 "Track_02" :Option%203 "Track_03")))

(event EventTick
  (params (DeltaSeconds :type Float%20%28single-precision%29)))

(event EventP1Scored
  (if (CallFunction|IsScoreDifferenceEven)
    (Default|QueueLayerModification (Actor|GetComponentbyClass (Variables|Default|GetLeftPaddle) "/Game/BpC_MusicTrack.BpC_MusicTrack_C") -1)
    (else
      (Default|QueueLayerModification (Actor|GetComponentbyClass (Variables|Default|GetPaddle) "/Game/BpC_MusicTrack.BpC_MusicTrack_C") 1))))

(event EventP2Scored
  (if (CallFunction|IsScoreDifferenceEven)
    (Default|QueueLayerModification (Actor|GetComponentbyClass (Variables|Default|GetPaddle) "/Game/BpC_MusicTrack.BpC_MusicTrack_C") -1)
    (else
      (Default|QueueLayerModification (Actor|GetComponentbyClass (Variables|Default|GetLeftPaddle) "/Game/BpC_MusicTrack.BpC_MusicTrack_C") 1))))

(fn ConstructionScript)

(fn IsScoreDifferenceEven
  (return (== (Math|Integer|%(Integer) (Math|Integer|Absolute(Integer) (- (Variables|Default|GetP2Score) (Variables|Default|GetP1Score))) 2) 0)))