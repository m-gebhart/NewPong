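; Music component that plays a layered, tempo-synced track from DT_MusicTracks, auto-starting Track_01 only on the owner named RightPaddle.
; It creates a 2D sound per layer, starts one at random and runs a looping bar timer derived from BPM.
; Layer requests, queued every five seconds, apply at bar end by adding one random unplayed layer; negative requests do nothing.
; Other events stop the track or restart it with all or some layers.
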(event Custom|InitializeTrack
  (params (Data%20Table%20Row%20Name :type Name))
  (bind _returnvalue (Utilities|GetDataTableRow "/Game/DT_MusicTracks.DT_MusicTracks" Data%20Table%20Row%20Name)
    (:then
      (Development|PrintString (Utilities|String|Append "Initializing " (.Name (Utilities|Struct|Breaks_MusicTrack _returnvalue))) true true "(R=0.000000,G=0.675000,B=0.184182,A=1.000000)")
      (Variables|Default|SetTrackInformation _returnvalue)
      (CallFunction|CalculateTactDuration)
      (CallFunction|GenerateLayers))
    (:RowNotFound
      (Development|PrintString (Utilities|String|Append "ERROR: CANNOT INITIALIZE TRACK WITH ROW NAME " (Utilities|String|ToString(Name) Data%20Table%20Row%20Name)) true true "(R=1.000000,G=0.037066,B=0.000000,A=1.000000)" 5.0))))

(event Custom|Generate%20Layers
  (for (_array_element _array_index) (.Layers (Utilities|Struct|Breaks_MusicTrack (Variables|Default|GetTrackInformation)))
    (bind _returnvalue (Audio|CreateSound2D _array_element (Variables|Default|GetAudioVolume) 1.0 0.0 0 false false))
    (Utilities|Array|Add (Variables|Default|GetSoundLayers) _returnvalue)
    (Utilities|Array|Add (Variables|Default|GetLayerIndicesNotPlayed) _array_index))
  (Variables|Default|SetOriginalLayerIndicesNotPlayed (Variables|Default|GetLayerIndicesNotPlayed))
  (CallFunction|PlayAmountOfLayers 1)
  (Utilities|FlowControl|Delay 5.0 :!label _label)
  (CallFunction|ModifyLayersonTact 1)
  (goto _label))

(event Custom|PlayFullTrack
  (CallFunction|StopTrack)
  (Variables|Default|SetLayerIndicesPlayed (Variables|Default|GetOriginalLayerIndicesNotPlayed))
  (CallFunction|StartLayerstoPlay))

(event Custom|PlayAmountOfLayers
  (params (Amount :type Integer))
  (bind _layerindicesnotplayed (Variables|Default|GetLayerIndicesNotPlayed))
  (CallFunction|StopTrack)
  (Utilities|Array|Shuffle (Variables|Default|GetLayerIndicesNotPlayed))
  (for _index (range 0 (- Amount 1))
    (Utilities|Array|Add (Variables|Default|GetLayerIndicesPlayed) (Utilities|Array|Get(acopy) _layerindicesnotplayed))
    (Utilities|Array|RemoveIndex _layerindicesnotplayed))
  (CallFunction|StartLayerstoPlay))

(event Custom|PrintLayerIndices
  (Development|PrintString (Utilities|String|Append "Layers played: " (Utilities|String|ToString(Integer) (Utilities|Array|Length (Variables|Default|GetLayerIndicesPlayed))) "        Layers not played: " (Utilities|String|ToString(Integer) (Utilities|Array|Length (Variables|Default|GetLayerIndicesNotPlayed))))))

(event Custom|StartLayersToPlay
  (Utilities|FlowControl|Delay (Variables|Default|GetTactDuration))
  (for _array_element (Variables|Default|GetLayerIndicesPlayed)
    (Audio|Components|Audio|Play (Utilities|Array|Get(acopy) (Variables|Default|GetSoundLayers) _array_element) 0.0))
  (bind _returnvalue (Utilities|Time|SetTimerbyEvent (delegate Custom|OnTactEnd) (Variables|Default|GetTactDuration) true))
  (Variables|Default|SetTactTimerHandle _returnvalue))

(event Custom|StopTrack
  (bind _tacttimerhandle (Variables|Default|GetTactTimerHandle))
  (if (Utilities|Time|IsValidTimerHandle _tacttimerhandle)
    (Utilities|Time|ClearandInvalidateTimerbyHandle _tacttimerhandle))
  (Variables|Default|SetLayerIndicesNotPlayed (Variables|Default|GetOriginalLayerIndicesNotPlayed))
  (bind _array_element (Utilities|Array|ForEachLoopwithBreak (Variables|Default|GetLayerIndicesPlayed))
    (:LoopBody
      (Audio|Components|Audio|Stop (Utilities|Array|Get(acopy) (Variables|Default|GetSoundLayers) _array_element)))
    (:Completed
      (Utilities|Array|Clear (Variables|Default|GetLayerIndicesPlayed)))))

(event Custom|AddLayer
  (bind _layerindicesnotplayed (Variables|Default|GetLayerIndicesNotPlayed))
  (bind _output (Utilities|Array|Get(acopy) _layerindicesnotplayed))
  (if (>= (Utilities|Array|Length (Variables|Default|GetLayerIndicesNotPlayed)) 1)
    (Utilities|Array|Shuffle _layerindicesnotplayed)
    (Utilities|Array|Add (Variables|Default|GetLayerIndicesPlayed) _output)
    (Audio|Components|Audio|Play (Utilities|Array|Get(acopy) (Variables|Default|GetSoundLayers) _output) 0.0)
    (Utilities|Array|RemoveIndex (Variables|Default|GetLayerIndicesNotPlayed))))

(event Custom|OnTactEnd
  (Math|Integer|CompareInt (Variables|Default|GetLayerModification)
    (:>
      (Variables|Default|SetLayerModification 0)
      (CallFunction|AddLayer))
    (:==
      _)
    (:<
      _))
  (Development|PrintString "Tact" true true "(R=0.000000,G=0.660000,B=1.000000,A=1.000000)" 0.1))

(event Custom|ModifyLayersOnTact
  (params (By :type Integer))
  (Variables|Default|SetLayerModification (+ (Variables|Default|GetLayerModification) By)))

(event EventBeginPlay
  (if (Utilities|Enum|Equal(Enum) (Utilities|GetObjectName (Components|GetOwner)) "RightPaddle")
    (CallFunction|InitializeTrack "Track_01")))

(fn CalculateTactDuration
  (bind _output_get (Variables|Default|SetTactDuration (* (/ 6e+01 (Math|Conversions|ToFloat(Integer) (Variables|Default|GetBPM))) (Math|Conversions|ToFloat(Integer) (Variables|Default|GetQuartersPerTact)))))
  (Development|PrintString (Utilities|String|ToString(Float) _output_get))
  (return))